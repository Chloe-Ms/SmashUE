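; BP_JammusEnergyBall is the energy ball actor for the Jammus character, which can be charged and then shot horizontally.
; ChargeStart and ChargeStop toggle visibility and the charging flag, while Tick scales the ball from zero to MaxScale by ChargeRatio until it moves.
; Shoot reveals it and sets direction, after which Tick moves it along X without sweep or delta-time scaling.
; A DestroyActor call is present but unconnected.
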(event EventChargeStart
  (Variables|Default|SetIsCharging true)
  (Rendering|SetActorHiddenInGame false))

(event EventChargeStop
  (Variables|Default|SetIsCharging false)
  (Rendering|SetActorHiddenInGame true))

(event EventTick
  (params (DeltaSeconds :type Float%20%28single-precision%29))
  (if (Variables|Default|GetIsMoving)
    (Transformation|SetActorLocation (+ (Transformation|GetActorLocation) (* (Math|Vector|MakeVector (Variables|Default|GetDirection) 0.0 0.0) (Variables|Default|GetMovementSpeed))) false false)
    (else
      (Transformation|SetActorScale3D (Math|Vector|Lerp(Vector) "0, 0, 0" (Variables|Default|GetMaxScale) (Variables|Default|GetChargeRatio))))))

(event EventShoot
  (params (Orientation :type Float%20%28single-precision%29))
  (Variables|Default|SetIsMoving true)
  (Variables|Default|SetDirection Orientation)
  (Rendering|SetActorHiddenInGame false))

(fn ConstructionScript)